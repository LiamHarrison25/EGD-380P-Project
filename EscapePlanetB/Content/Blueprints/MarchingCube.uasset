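; Marching cubes Blueprint that builds a procedural mesh with collision over a scaled 3D grid at BeginPlay.
; Each cell's corners get cached binary values from a height-based threshold, drawn as debug points.
; The eight values form a case index into a data table of triangle indices.
; Each cell becomes its own mesh section, using fixed edge points as vertices without interpolation.
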(event `Binary`
  (bind _updatedvertex (`self.updatedVertex`))
  (bind _cornermap (`self.cornerMap`))
  (for _array_element (`self.updatedVertex`)
    (bind _returnvalue (`KismetMathLibrary.Conv_IntToDouble` (`BlueprintMapLibrary.Map_Find` (`self.cornerMap`) _array_element)))
    (`KismetSystemLibrary.DrawDebugPoint` _array_element 10.0 (`KismetMathLibrary.MakeColor` _returnvalue _returnvalue _returnvalue) 30.0)
    (bind _returnvalue_2 (`|GetDataTableRow` "/Game/Data/MarchingCubes_DT.MarchingCubes_DT" (`KismetStringLibrary.Conv_StringToName` (`KismetStringLibrary.Conv_IntToString` (+ (+ (`BlueprintMapLibrary.Map_Find` _cornermap (`|GetArrayItem` _updatedvertex)) (* (`BlueprintMapLibrary.Map_Find` _cornermap (`|GetArrayItem` _updatedvertex 1)) 2) (* (`BlueprintMapLibrary.Map_Find` _cornermap (`|GetArrayItem` _updatedvertex 2)) 4) (* (`BlueprintMapLibrary.Map_Find` _cornermap (`|GetArrayItem` _updatedvertex 3)) 8) (* (`BlueprintMapLibrary.Map_Find` _cornermap (`|GetArrayItem` _updatedvertex 4)) 16) (* (`BlueprintMapLibrary.Map_Find` _cornermap (`|GetArrayItem` _updatedvertex 5)) 32) (* (`BlueprintMapLibrary.Map_Find` _cornermap (`|GetArrayItem` _updatedvertex 6)) 64) (* (`BlueprintMapLibrary.Map_Find` _cornermap (`|GetArrayItem` _updatedvertex 7)) 128)) 1))))
      (:`then`
        (set `self.Out Row Triangle Vertices_0` (break `/Game/Blueprints/MarchingArray` _returnvalue_2))))))

(event `self.ReceiveBeginPlay`
  (bind _grid_size (`self.Grid Size`))
  (bind _scale (`self.Scale`))
  (bind _scale_2 (`self.Scale`))
  (bind _updatededge (`self.updatedEdge`))
  (bind _updatedvertex (`self.updatedVertex`))
  (bind _cornermap (`self.cornerMap`))
  (for _index (range (+ _grid_size 1))
    (for _index_2 (range (+ _grid_size 1))
      (for _index_3 (range (+ _grid_size 1))
        (for (_array_element _array_index) (`self.EdgeData`)
          (bind _returnvalue (* _index 100.0))
          (bind _returnvalue_2 (* _index_2 100.0))
          (bind _returnvalue_3 (* _index_3 100.0))
          (`KismetArrayLibrary.Array_Set` _updatededge _array_index (`KismetMathLibrary.MakeVector` (* (+ _returnvalue (.x _array_element)) _scale_2) (* (+ _returnvalue_2 (.y _array_element)) _scale_2) (* (+ _returnvalue_3 (.z _array_element)) _scale_2))))
        (for (_array_element_2 _array_index_2) (`self.VertexData`)
          (`KismetArrayLibrary.Array_Set` _updatedvertex _array_index_2 (`KismetMathLibrary.MakeVector` (* (+ _returnvalue (.x _array_element_2)) _scale) (* (+ _returnvalue_2 (.y _array_element_2)) _scale) (* (+ _returnvalue_3 (.z _array_element_2)) _scale))))
        (for _array_element_3 _updatedvertex
          (if (not (`.ReturnValue` (`BlueprintMapLibrary.Map_Find` _cornermap _array_element_3)))
            (bind _z (.z _array_element_3))
            (`BlueprintMapLibrary.Map_Add` _cornermap (`KismetMathLibrary.MakeVector` (.x _array_element_3) (.y _array_element_3) _z) (`KismetMathLibrary.Clamp` (`KismetMathLibrary.FTrunc` (* _z (`KismetMathLibrary.DegSin` 1.0))) 0 1))))
        (`self.Binary`)
        (bind _result (`/Engine/EditorBlueprintResources/StandardMacros.IncrementInt` (`self.Section Index`))
          (:`  `
            (`ProceduralMeshComponent.CreateMeshSection_LinearColor` :`self` (`self.ProceduralMesh`) :`SectionIndex` _result :`Vertices` _updatededge :`Triangles` (`self.Out Row Triangle Vertices_0`) :`bCreateCollision` true)))))))

(fn `UserConstructionScript`)